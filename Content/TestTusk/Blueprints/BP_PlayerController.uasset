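; Player controller that registers the default Enhanced Input mapping and toggles the pause menu.
; On BeginPlay it adds IMC_Default to the local player's input subsystem.
; IA_Pause creates and shows WBP_PauseGame, pauses the game and enables the cursor with Game and UI input.
; Pressing it while paused removes the stored widget, unpauses and restores game-only input with a hidden cursor.
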(event Input|EnhancedActionEvents|EnhancedInputActionIA_Pause
  (params (ActionValue :type Boolean) (ElapsedSeconds :type Float%20%28double-precision%29) (TriggeredSeconds :type Float%20%28double-precision%29) (InputAction :type Input%20Action%20Object%20Reference :default "/Game/TestTusk/Input/Actions/IA_Pause.IA_Pause"))
  (bind _self self)
  (:Started
    (if (Game|IsGamePaused)
      (bind _pause_ref (Variables|Default|GetPause%20Ref)
        (:then
          (Widget|RemovefromParent _pause_ref)
          (Game|SetGamePaused false)
          (Input|SetInputModeGameOnly _self false)
          (Variables|Default|SetbShowMouseCursor false))
        (:else))
      (else
        (bind _returnvalue (UserInterface|CreateWidget "/Game/TestTusk/UI/WBP_PauseGame.WBP_PauseGame_C"))
        (bind _output_get (Variables|Default|SetPause%20Ref _returnvalue))
        (UserInterface|Viewport|AddtoViewport _output_get 0)
        (Game|SetGamePaused true)
        (Input|SetInputModeGameandUI _self 0 "DoNotLock" false false)
        (Variables|Default|SetbShowMouseCursor true)))))

(event EventBeginPlay
  (bind _self self)
  (bind _returnvalue (PlayerController|LocalPlayerSubsystems|GetEnhancedInputLocalPlayerSubsystem _self))
  (Utilities|IsValid _returnvalue
    (:Is%20Valid
      (Input|AddMappingContext _returnvalue "/Game/TestTusk/Input/IMC_Default.IMC_Default" 0 "(bIgnoreAllPressedKeysUntilRelease=True,bForceImmediately=False)"))))

(fn ConstructionScript)